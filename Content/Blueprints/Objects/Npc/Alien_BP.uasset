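; Alien NPC that wanders, enters combat when shot by the player and dies once its randomly rolled hit points run out.
; BeginPlay feeds range, wait time and speed bias settings into a movement component that drives the NPC.
; Capsule overlaps with player bullets decrement HP and switch state, with death interrupting movement before a delayed switch to the dead animation.
; The construction script assigns a Paper2D flipbook as its visual representation.
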(event OnComponentBeginOverlap(Capsule)
  (params (OverlappedComponent :type Primitive%20Component%20Object%20Reference) (OtherActor :type Actor%20Object%20Reference) (OtherComp :type Primitive%20Component%20Object%20Reference) (OtherBodyIndex :type Integer) (bFromSweep :type Boolean) (SweepResult :type Hit%20Result%20Structure%20%28by%20ref%29))
  (Utilities|Casting|CastToPlayerBullet_BP OtherActor)
  (bind _result (Math|Integer|DecrementInt (Variables|Default|Gethp))
    (:%20%20
      (if (>= _result 0)
        (Class|BaseNpc|SwitchState "ENpcCombat")
        (else
          (Class|BaseNpc|SwitchState "ENpcDying")
          (Utilities|FlowControl|Delay 0.1)
          (Default|Interrupt (Variables|Default|GetMovementComponent))
          (Utilities|FlowControl|Delay 0.5)
          (Class|BaseNpc|SetAnimationState "ENpcDeadAnim")
          (Class|BaseNpc|SwitchAnimation))))))

(event EventBeginPlay
  (Default|Init (Variables|Default|GetMovementComponent) (Variables|Default|GetDefaultSceneRoot) "0, 0,-90.000000" (Variables|Default|GetcombatSpeedBias) (Math|Conversions|ToVector(Vector2D) (Variables|Default|GetmaxMovementRange) 1.0) (Math|Conversions|ToVector(Vector2D) (Variables|Default|GetminMovementRange) 1.0) (Variables|Default|GetwanderWaitTime) self)
  (Variables|Default|Sethp (Math|Random|RandomIntegerinRange (Variables|Default|GetMinHpValue) (Variables|Default|GetMaxHpValue))))

(event Collision|EventActorBeginOverlap
  (params (OtherActor :type Actor%20Object%20Reference)))

(event EventTick
  (params (DeltaSeconds :type Float%20%28single-precision%29)))

(fn ConstructionScript
  (Variables|Default|SetnpcRepresentation (Variables|Default|GetPaperFlipbook)))