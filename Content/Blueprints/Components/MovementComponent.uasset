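; Movement component that makes an NPC's scene component roam endlessly between random points within configured bounds.
; Init starts a Move loop that sets speed by NPC state, flips between normal and mirrored rotation by X direction, then tweens via MoveComponentTo.
; On arrival, idle or wandering NPCs pause before moving again, while combat uses scaled speed and a short delay.
; Random pure nodes re-roll per execution step, so facing can mismatch the target.
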(event Custom|Interrupt
  (bind _minvalues (Variables|Default|GetMinValues))
  (bind _maxvalues (Variables|Default|GetMaxValues))
  (bind _movednpc (Variables|Default|GetMovedNpc))
  (bind (_x _y _z) (Math|Vector|BreakVector _minvalues))
  (bind (_x_2 _y_2 _z_2) (Math|Vector|BreakVector _maxvalues))
  (bind _returnvalue (Math|Random|RandomFloatinRange _z _z_2))
  (bind _returnvalue_2 (Math|Random|RandomFloatinRange _x _x_2))
  (bind _returnvalue_3 (Math|Random|RandomFloatinRange _y _y_2))
  (bind _returnvalue_4 (Math|Vector|MakeVector _returnvalue_2 _returnvalue_3 _returnvalue))
  (Components|MoveComponentTo (Variables|Default|GetComponentToMove) _returnvalue_4 (Variables|Default|GetCurrentRot) false false (/ (Math|Vector|VectorLength (- _returnvalue_4 (Transformation|GetActorLocation (Components|GetOwner)))) (Variables|Default|GetCurrentSpeed)) false) ; enters at Stop
)

(event Custom|Move
  (bind _returnvalue (Components|GetOwner))
  (bind _minvalues (Variables|Default|GetMinValues))
  (bind _maxvalues (Variables|Default|GetMaxValues))
  (bind _movednpc (Variables|Default|GetMovedNpc))
  (bind (_x _y _z) (Math|Vector|BreakVector _minvalues))
  (bind _returnvalue_2 (Transformation|GetActorLocation _returnvalue))
  (bind (_x_2 _y_2 _z_2) (Math|Vector|BreakVector _maxvalues))
  (bind _returnvalue_3 (Math|Random|RandomFloatinRange _z _z_2))
  (bind _returnvalue_4 (Math|Random|RandomFloatinRange _x _x_2))
  (bind _returnvalue_5 (Math|Random|RandomFloatinRange _y _y_2))
  (bind _returnvalue_6 (Math|Vector|MakeVector _returnvalue_4 _returnvalue_5 _returnvalue_3))
  (bind _returnvalue_7 (- _returnvalue_6 _returnvalue_2))
  (bind _x_3 (Math|Vector|BreakVector _returnvalue_7))
  (CallFunction|SetMovementSpeed)
  (Development|PrintString (Utilities|String|Append (Utilities|String|ToString(Float) (.X (Math|Vector|BreakVector _returnvalue_6))) " ||| " (Utilities|String|ToString(Float) _x_3)))
  (CallFunction|SetMovementBasedRotation _x_3)
  (Components|MoveComponentTo (Variables|Default|GetComponentToMove) _returnvalue_6 (Variables|Default|GetCurrentRot) false false (/ (Math|Vector|VectorLength _returnvalue_7) (Variables|Default|GetCurrentSpeed)) false)
  (Utilities|IsValid (Variables|Default|GetMovedNpc)
    (:Is%20Valid
      (bind _returnvalue_8 (Class|BaseNpc|GetState _movednpc))
      (switch Utilities|FlowControl|Switch|SwitchonENpcStatus _returnvalue_8
        (:ENpcIdle
          (Class|BaseNpc|SwitchState _movednpc "ENpcIdle" :!label _label)
          (Utilities|FlowControl|Delay (Variables|Default|GetWaitTime))
          (bind _returnvalue_9 (Class|BaseNpc|GetState (Variables|Default|GetMovedNpc)))
          (switch Utilities|FlowControl|Switch|SwitchonENpcStatus _returnvalue_9
            (:ENpcIdle
              (Class|BaseNpc|SwitchState (Variables|Default|GetMovedNpc) "ENpcWander"))
            (:ENpcCombat
              _))
          (CallFunction|Move))
        (:ENpcCombat
          (Utilities|FlowControl|Delay 0.4 :!label _label_2)
          (CallFunction|Move))
        (:ENpcWander
          (goto _label))
        (:ENpcSpawned
          (goto _label_2))))
    (:Is%20Not%20Valid
      (goto _label_2))))

(event EventBeginPlay)

(event EventTick
  (params (DeltaSeconds :type Float%20%28single-precision%29)))

(fn MoveComponent)

(fn Init
  (params (SceneComp :type Scene%20Component%20Object%20Reference) (Rotator :type Rotator) (TimeBias :type Float%20%28single-precision%29) (MaximalMovementRange :type Vector) (MinimalMovementRange :type Vector) (TimeDelay :type Float%20%28single-precision%29) (NpcRef :type Base%20Npc%20Object%20Reference))
  (Variables|Default|SetRelativeRot Rotator)
  (Variables|Default|SetComponentToMove SceneComp)
  (Variables|Default|SetAvgTime TimeBias)
  (Variables|Default|SetMinValues MinimalMovementRange)
  (Variables|Default|SetMaxValues MaximalMovementRange)
  (bind _result (Math|Float|NegateFloat (.Roll (Math|Rotator|BreakRotator (Variables|Default|GetRelativeRot))))
    (:%20%20
      (Variables|Default|SetMirroredRot (Math|Rotator|MakeRotator _result (.Pitch (Math|Rotator|BreakRotator (Variables|Default|GetRelativeRot))) -1.8e+02))
      (Variables|Default|SetWaitTime TimeDelay)
      (Variables|Default|SetMovedNpc NpcRef)
      (CallFunction|Move))))

(fn SetMovementSpeed
  (Utilities|IsValid (Variables|Default|GetMovedNpc)
    (:Is%20Valid
      (bind _returnvalue (Class|BaseNpc|GetState (Variables|Default|GetMovedNpc)))
      (switch Utilities|FlowControl|Switch|SwitchonENpcStatus _returnvalue
        (:ENpcIdle
          (Variables|Default|SetCurrentSpeed (Variables|Default|GetBaseValue) :!label _label))
        (:ENpcCombat
          (Variables|Default|SetCurrentSpeed (* (Variables|Default|GetBaseValue) (Variables|Default|GetAvgTime))))
        (:ENpcWander
          (goto _label))
        (:ENpcDying
          (goto _label))
        (:ENpcSpawned
          (goto _label)))
      (return))
    (:Is%20Not%20Valid
      (Variables|Default|SetCurrentSpeed (Variables|Default|GetBaseValue))
      (return))))

(fn SetMovementBasedRotation
  (params (directionVal :type Float%20%28single-precision%29))
  (bind _relativerot (Variables|Default|GetRelativeRot))
  (Math|Float|CompareFloat directionVal 0.0
    (:>
      (Variables|Default|SetCurrentRot _relativerot))
    (:==
      (Variables|Default|SetCurrentRot _relativerot))
    (:<
      (Variables|Default|SetCurrentRot (Variables|Default|GetMirroredRot))))
  (Transformation|SetRelativeRotation (Variables|Default|GetComponentToMove) (Variables|Default|GetCurrentRot) false false)
  (return))