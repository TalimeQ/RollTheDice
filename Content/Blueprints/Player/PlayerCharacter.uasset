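; Player character Blueprint that uses a flipbook as its visual representation and handles shooting.
; On a shoot intent it disables movement, switches to the shooting animation, and after a short delay spawns a PlayerBullet_BP at Arrow1's transform with a fixed +X direction.
; A second delay then sets the idle state and restores walking; the Shoot function is an empty stub.
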(event Collision|EventActorBeginOverlap
  (params (OtherActor :type Actor%20Object%20Reference)))

(event EventTick
  (params (DeltaSeconds :type Float%20%28single-precision%29)))

(event EventBeginPlay
  (Variables|Default|SetplayerRepresentation (Variables|Default|GetPlayerFlipbook)))

(event EventProcessIntentShoot
  (bind _charactermovement (Variables|Character|GetCharacterMovement))
  (Pawn|Components|CharacterMovement|DisableMovement _charactermovement)
  (Class|PlayerAgentCharacter|SetAnimationState "EShooting")
  (Class|PlayerAgentCharacter|ChangeAnimation)
  (Utilities|FlowControl|Delay 0.2)
  (bind _returnvalue (Game|SpawnActorfromClass "/Game/Blueprints/Objects/PlayerBullet_BP.PlayerBullet_BP_C" (Transformation|GetWorldTransform (Variables|Default|GetArrow1)) "AlwaysSpawn" 0 0))
  (Class|BaseProjectine|SetupBullet _returnvalue "1.000000,0.000000, 0" 2.5e+02 1)
  (Utilities|FlowControl|Delay 0.2)
  (Class|PlayerAgentCharacter|SetAnimationState "EIdle")
  (Pawn|Components|CharacterMovement|SetMovementMode _charactermovement "MOVE_Walking" 0))

(fn ConstructionScript)

(fn Shoot)